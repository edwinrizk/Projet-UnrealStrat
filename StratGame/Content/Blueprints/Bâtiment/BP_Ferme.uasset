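; BP_Ferme is a farm building that is built over time and then raises food yield and housing capacity.
; Its ConstructionFerme event loops on a one-second Delay, adding the dedicated production to its construction points until they reach the maximum.
; On completion, the AddForReference helper adds the farm's food and housing bonuses to the passed-in current values through float references, and a completion message is printed.
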(event Custom|Construction%20Ferme
  (params (RdmNourActu :type Float%20%28double-precision%29%20%28by%20ref%29) (HabitationActuel :type Float%20%28double-precision%29%20%28by%20ref%29) (ProdDédié :type Float%20%28double-precision%29))
  (if (< (Variables|Default|GetPointConstruction) (Variables|Default|GetPointConstructionMax)) :!label _label
    (Variables|Default|SetPointConstruction (+ (Variables|Default|GetPointConstruction) ProdDédié))
    (Utilities|FlowControl|Delay 1.0)
    (goto _label)
    (else
      (Utilities|AddforReference RdmNourActu (Variables|Default|GetRdmNourPlus)
        (:%20%20
          (Utilities|AddforReference HabitationActuel (Variables|Default|GetHabitationPlus)
            (:%20%20
              (Development|PrintText "Construction terminée"))))))))

(event Collision|EventActorBeginOverlap
  (params (OtherActor :type Actor%20Object%20Reference)))

(event EventTick
  (params (DeltaSeconds :type Float%20%28single-precision%29)))

(fn ConstructionScript)