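; BP_QuartierGeneral is a headquarters building that produces four strategic resources: gold, iron, horses and saltpetre.
; Tick chains IncrementRessource for each, but only on frames whose DeltaSeconds reaches one second, as no timer accumulates.
; IncrementRessource adds the yield through by-reference AddForReference only when the resource equals StockRessStrat, and its output fires only then.
; Clicking the actor prints a placeholder "Hello".
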(event EventTick
  (params (DeltaSeconds :type Float%20%28single-precision%29))
  (if (>= DeltaSeconds 1.0)
    (Utilities|IncrementRessource (Variables|Default|GetOrs) (Variables|Default|GetRendementOr)
      (:Sortie
        (Utilities|IncrementRessource (Variables|Default|GetFers) (Variables|Default|GetRendementFer)
          (:Sortie
            (Utilities|IncrementRessource (Variables|Default|GetChevaux) (Variables|Default|GetRendementChevaux)
              (:Sortie
                (Utilities|IncrementRessource (Variables|Default|GetSalpêtre) (Variables|Default|GetRendementSalpêtre))))))))))

(event Collision|EventActorBeginOverlap
  (params (OtherActor :type Actor%20Object%20Reference)))

(event MouseInput|EventActorOnClicked
  (params (ButtonPressed :type Key%20Structure :default "None"))
  (Development|PrintText "Hello"))

(fn ConstructionScript)