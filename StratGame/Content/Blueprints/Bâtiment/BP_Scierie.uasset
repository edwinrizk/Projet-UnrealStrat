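; Sawmill (Scierie) building Blueprint that handles its construction and the production yield bonus it grants.
; The ConstructionScierie event runs a macro that adds dedicated production to construction points every second, looping only while points equal the maximum.
; After the loop, a by-reference float helper adds the building's bonus to the supplied current yield and a completion message prints.
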(event Custom|Construction%20Scierie
  (params (RdmProdActu :type Float%20%28double-precision%29%20%28by%20ref%29) (ProdDédié :type Float%20%28double-precision%29))
  (Utilities|ConstructionMacro RdmProdActu ProdDédié))

(event Collision|EventActorBeginOverlap
  (params (OtherActor :type Actor%20Object%20Reference)))

(event EventTick
  (params (DeltaSeconds :type Float%20%28single-precision%29)))

(fn ConstructionScript)