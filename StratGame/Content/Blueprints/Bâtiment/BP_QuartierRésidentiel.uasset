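; Residential district building (Quartier Résidentiel) that adds housing to a headquarters (QG) once its construction completes.
; ConstructionQR runs a one-second Delay loop, adding the QG's production rate divided by its active construction count until the maximum is reached.
; On completion it increases the QG's Habitations by reference, prints a message and decrements that count.
; BeginPlay initializes health (Vie).
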(event Custom|Construction%20QR
  (params (QG :type BP%20Quartier%20General%20Object%20Reference%20%28by%20ref%29))
  (bind _nbconstruction (Variables|/Game/Blueprints/Bâtiment/BP_QuartierGeneral.BP_QuartierGeneral_C|GetNbConstruction QG))
  (if (< (Variables|Default|GetPointConstruction) (Variables|Default|GetPointConstructionMax)) :!label _label
    (Variables|Default|SetPointConstruction (+ (Variables|Default|GetPointConstruction) (/ (Variables|/Game/Blueprints/Bâtiment/BP_QuartierGeneral.BP_QuartierGeneral_C|GetRendementProduction QG) _nbconstruction)))
    (Utilities|FlowControl|Delay 1.0)
    (goto _label)
    (else
      (Utilities|AddforReference (Variables|/Game/Blueprints/Bâtiment/BP_QuartierGeneral.BP_QuartierGeneral_C|GetHabitations QG) (Variables|Default|GetHabitationPlus)
        (:%20%20
          (Development|PrintText "Construction terminée")
          (Math|Integer|DecrementInt _nbconstruction))))))

(event EventBeginPlay
  (Variables|Default|SetVie 2e+02))

(fn ConstructionScript
  (|CallParentFunction))