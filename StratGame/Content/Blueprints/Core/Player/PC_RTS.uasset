(event Custom|ActorSelected
  (params (Actor :type Actor%20Object%20Reference))
  (CallFunction|DeselectAllActors)
  (Utilities|Array|Add (Variables|Default|GetSelectedActor) Actor))

(event Custom|DeselectAllActors
  (for _array_element (Variables|Default|GetSelectedActor)
    (if (Utilities|DoesObjectImplementInterface _array_element "/Game/Blueprints/Core/Bâtiment/BPI_SelectionEvent.BPI_SelectionEvent_C")
      (Class|BPISelectionEvent|DeselectThis(Message) _array_element)))
  (Utilities|Array|Clear (Variables|Default|GetSelectedActor)))

(event EventTick
  (params (DeltaSeconds :type Float%20%28single-precision%29)))

(event EventBeginPlay
  (bind _returnvalue (Actor|GetActorOfClass "/Game/Blueprints/Bâtiment/BP_QuartierGeneral.BP_QuartierGeneral_C"))
  (Variables|Default|SetQG _returnvalue))

(event Input|ActionEvents|InputActionMouseAction
  (params (Key :type Key%20Structure :default "None"))
  (bind _hitresult (Game|Player|GetHitResultUnderCursorbyChannel "TraceTypeQuery1" true))
  (bind _selectedactor (Variables|Default|GetSelectedActor))
  (:Released
    (if (Utilities|Array|IsNotEmpty _selectedactor)
      (for _array_element _selectedactor
        (if (Utilities|DoesObjectImplementInterface _array_element "/Game/Blueprints/Core/Troupes/Guerrier/BPI_UnitActions.BPI_UnitActions_C")
          (Class|BPIUnitActions|MovetoLocation(Message) _array_element (.location _hitresult))
          (Niagara|SpawnSystematLocation "/Game/Blueprints/Core/Player/NS_ClickIndicator.NS_ClickIndicator" (.location _hitresult)))))))

(event Input|ActionEvents|InputActionAjoutCM
  (params (Key :type Key%20Structure :default "None"))
  (bind _qg (Variables|Default|GetQG))
  (:Pressed
    (bind _returnvalue (Game|SpawnActorfromClass "/Game/Blueprints/Bâtiment/BP_CampMilitaire.BP_CampMilitaire_C" (Math|Transform|MakeTransform (.location (.HitResult (Game|Player|GetHitResultUnderCursorbyChannel "TraceTypeQuery1" true))) "0, 0, 0" "1.000000,1.000000,1.000000") "Undefined" "MultiplyWithRoot" 0 0))
    (if (<= (/ (Variables|/Game/Blueprints/Bâtiment/BP_QuartierGeneral.BP_QuartierGeneral_C|GetPopulation _qg) (Variables|/Game/Blueprints/Bâtiment/BP_QuartierGeneral.BP_QuartierGeneral_C|GetNbCM _qg)) 5)
      (Utilities|RadiusVerif _returnvalue)
      (else
        (Actor|DestroyActor _returnvalue)
        (Development|PrintText "Population trop faible.")))))

(event Input|ActionEvents|InputActionAjoutMine
  (params (Key :type Key%20Structure :default "None"))
  (:Pressed
    (bind _returnvalue (Game|SpawnActorfromClass "/Game/Blueprints/Bâtiment/BP_Mine.BP_Mine_C" (Math|Transform|MakeTransform (.location (.HitResult (Game|Player|GetHitResultUnderCursorbyChannel "TraceTypeQuery1" true))) "0, 0, 0" "1.000000,1.000000,1.000000") "Undefined" "MultiplyWithRoot" 0 0))
    (Utilities|RadiusVerif _returnvalue)))

(event Input|ActionEvents|InputActionAjoutAP
  (params (Key :type Key%20Structure :default "None"))
  (:Pressed
    (bind _returnvalue (Game|SpawnActorfromClass "/Game/Blueprints/Bâtiment/BP_AvantPoste.BP_AvantPoste_C" (Math|Transform|MakeTransform (.location (.HitResult (Game|Player|GetHitResultUnderCursorbyChannel "TraceTypeQuery1" true))) "0, 0, 0" "1.000000,1.000000,1.000000") "Undefined" "MultiplyWithRoot" 0 0))
    (Utilities|RadiusVerif _returnvalue)))

(event Input|ActionEvents|InputActionAjoutFerme
  (params (Key :type Key%20Structure :default "None"))
  (:Pressed
    (bind _returnvalue (Game|SpawnActorfromClass "/Game/Blueprints/Bâtiment/BP_Ferme.BP_Ferme_C" (Math|Transform|MakeTransform (.location (.HitResult (Game|Player|GetHitResultUnderCursorbyChannel "TraceTypeQuery1" true))) "0, 0, 0" "1.000000,1.000000,1.000000") "Undefined" "MultiplyWithRoot" 0 0))
    (Utilities|RadiusVerif _returnvalue)))

(event Input|ActionEvents|InputActionAjoutScierie
  (params (Key :type Key%20Structure :default "None"))
  (:Pressed
    (bind _returnvalue (Game|SpawnActorfromClass "/Game/Blueprints/Bâtiment/BP_Scierie.BP_Scierie_C" (Math|Transform|MakeTransform (.location (.HitResult (Game|Player|GetHitResultUnderCursorbyChannel "TraceTypeQuery1" true))) "0, 0, 0" "1.000000,1.000000,1.000000") "Undefined" "MultiplyWithRoot" 0 0))
    (Utilities|RadiusVerif _returnvalue)))

(event Input|ActionEvents|InputActionAjoutQR
  (params (Key :type Key%20Structure :default "None"))
  (:Pressed
    (bind _returnvalue (Game|SpawnActorfromClass "/Game/Blueprints/Bâtiment/BP_QuartierRésidentiel.BP_QuartierRésidentiel_C" (Math|Transform|MakeTransform (.location (.HitResult (Game|Player|GetHitResultUnderCursorbyChannel "TraceTypeQuery1" true))) "0, 0, 0" "1.000000,1.000000,1.000000") "Undefined" "MultiplyWithRoot" 0 0))
    (Utilities|RadiusVerif _returnvalue)))

(event Input|AxisEvents|InputAxismoveForward
  (params (AxisValue :type Float%20%28single-precision%29))
  (Pawn|Input|AddMovementInput (Pawn|GetControlledPawn) (Math|Vector|GetForwardVector (Math|Rotator|MakeRotator 0.0 0.0 (.yaw (Pawn|GetControlRotation :!class /Script/Engine.Controller)))) (Math|Float|SelectFloat AxisValue (Variables|Default|GetMouseForwardScale) (!= AxisValue 0.0)) false))

(event Input|AxisEvents|InputAxisMoveRIght
  (params (AxisValue :type Float%20%28single-precision%29))
  (Pawn|Input|AddMovementInput (Pawn|GetControlledPawn) (Math|Vector|GetRightVector (Math|Rotator|MakeRotator 0.0 0.0 (.yaw (Pawn|GetControlRotation :!class /Script/Engine.Controller)))) (Math|Float|SelectFloat AxisValue (Variables|Default|GetMouseRightScale) (!= AxisValue 0.0)) false))

(event Input|AxisEvents|InputAxisMouseMovement
  (params (AxisValue :type Float%20%28single-precision%29))
  (bind _locationy (Game|Player|GetMousePosition))
  (bind _returnvalue (Viewport|GetViewportSize))
  (bind _returnvalue_2 (Viewport|GetViewportSize))
  (bind _locationx (Game|Player|GetMousePosition))
  (bind _returnvalue_3 (Viewport|GetViewportSize))
  (bind (_locationx_2 _locationy_2) (Game|Player|GetMousePosition))
  (bind _returnvalue_4 (/ _locationx (.x _returnvalue_3)))
  (bind _returnvalue_5 (/ _locationy (.y _returnvalue)))
  (Development|PrintString (Utilities|String|Append (Utilities|String|ToString(Float) (/ _locationx_2 (.x _returnvalue_2))) "" (Utilities|String|ToString(Float) (/ _locationy_2 (.y _returnvalue_2)))) true true "(R=0.000000,G=0.660000,B=1.000000,A=1.000000)" 0.0)
  (Variables|Default|SetMouseRightScale (Math|Float|SelectFloat -1.0 (Math|Float|SelectFloat 1.0 0.0 (> _returnvalue_4 (- 1.0 (Variables|Default|GetviewPortEdgeTreshhold)))) (< _returnvalue_4 (Variables|Default|GetviewPortEdgeTreshhold))))
  (Variables|Default|SetMouseForwardScale (Math|Float|SelectFloat 1.0 (Math|Float|SelectFloat -1.0 0.0 (> _returnvalue_5 (- 1.0 (Variables|Default|GetviewPortEdgeTreshhold)))) (< _returnvalue_5 (Variables|Default|GetviewPortEdgeTreshhold)))))

(fn ConstructionScript)