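; Warrior troop unit that either follows player move orders or, once flagged as an enemy, attacks buildings.
; Player units use AI MoveTo on command and hide their decal when deselected.
; SetEnnemy sends the unit to a random building from the supplied array, damages its Vie every second, destroys it at zero, then loops to another target.
; The validity check runs on the previous Index, before the random pick.
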(event Custom|Set%20Ennemy
  (params (Bâtiments :type Array%20of%20BP%20Bâtiment%20Object%20References))
  (Variables|Default|SetisEnnemy true)
  (if (Math|Boolean|ANDBoolean (Utilities|Array|IsNotEmpty Bâtiments) (not (Game|IsActorBeingDestroyed (Utilities|Array|Get(acopy) Bâtiments (Variables|Default|Getindex)))) (Utilities|IsValid (Utilities|Array|Get(acopy) Bâtiments (Variables|Default|Getindex)))) :!label _label
    (Variables|Default|Setindex (Math|Random|RandomInteger (Utilities|Array|Length Bâtiments)))
    (AI|AIMoveTo self (Transformation|GetActorLocation (Utilities|Array|Get(acopy) Bâtiments (Variables|Default|Getindex))) (Utilities|Array|Get(acopy) Bâtiments (Variables|Default|Getindex)) (Variables|/Game/Blueprints/Core/Bâtiment/BP_Bâtiment.BP_Bâtiment_C|GetAcceptanceRadius (Utilities|Array|Get(acopy) Bâtiments (Variables|Default|Getindex))) false
      (:OnSuccess
        (if (not (Game|IsActorBeingDestroyed (Utilities|Array|Get(acopy) Bâtiments (Variables|Default|Getindex))))
          (Utilities|FlowControl|Delay 1.0 :!label _label_2)
          (if (<= (Variables|/Game/Blueprints/Core/Bâtiment/BP_Bâtiment.BP_Bâtiment_C|GetVie (Utilities|Array|Get(acopy) Bâtiments (Variables|Default|Getindex))) 0.0)
            (if (not (Game|IsActorBeingDestroyed (Utilities|Array|Get(acopy) Bâtiments (Variables|Default|Getindex))))
              (Actor|DestroyActor (Utilities|Array|Get(acopy) Bâtiments (Variables|Default|Getindex)))
              (Utilities|Array|RemoveItem Bâtiments (Utilities|Array|Get(acopy) Bâtiments (Variables|Default|Getindex)))
              (Development|PrintText "Bâtiment détruit !")
              (goto _label)
              (else
                (goto _label)))
            (else
              (Variables|/Game/Blueprints/Core/Bâtiment/BP_Bâtiment.BP_Bâtiment_C|SetVie (Utilities|Array|Get(acopy) Bâtiments (Variables|Default|Getindex)) (- (Variables|/Game/Blueprints/Core/Bâtiment/BP_Bâtiment.BP_Bâtiment_C|GetVie (Utilities|Array|Get(acopy) Bâtiments (Variables|Default|Getindex))) 5.0))
              (Development|PrintText "Bâtiment attaqué !")
              (goto _label_2)))
          (else
            (goto _label))))
      (:OnFail
        (goto _label)))))

(event EventBeginPlay
  (Variables|Default|SetVie 5e+01))

(event Collision|EventActorBeginOverlap
  (params (OtherActor :type Actor%20Object%20Reference)))

(event EventTick
  (params (DeltaSeconds :type Float%20%28single-precision%29)))

(event EventDeselectThis
  (bind _decal (Variables|Default|GetDecal))
  (Development|SetHiddeninGame _decal true false)
  (Rendering|SetVisibility _decal false false))

(event EventMovetoLocation
  (params (NewLocation :type Vector :default "0, 0, 0"))
  (if (not (Variables|Default|GetisEnnemy))
    (AI|AIMoveTo self NewLocation 0 5e+01 false)))

(fn ConstructionScript)